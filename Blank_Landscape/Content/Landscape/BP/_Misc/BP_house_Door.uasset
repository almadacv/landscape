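; BP_house_Door is a house door that swings open when the third-person character enters its Box trigger.
; The overlap changes TargetAngle from zero to a fixed open angle, and nothing in the graph resets it to close the door.
; Tick rotates DoorA's relative yaw at Speed, signed by current minus target yaw, then snaps it to TargetAngle once within Threshold.
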(event OnComponentBeginOverlap(Box)
  (params (OverlappedComponent :type Primitive%20Component%20Object%20Reference) (OtherActor :type Actor%20Object%20Reference) (OtherComp :type Primitive%20Component%20Object%20Reference) (OtherBodyIndex :type Integer) (bFromSweep :type Boolean) (SweepResult :type Hit%20Result%20Structure%20%28by%20ref%29))
  (Utilities|Casting|CastToBP_ThirdPersonCharacter OtherActor)
  (if (and (== (Variables|Default|GetTarget_Angle) 0.0) (!= OtherComp (Variables|Default|GetDoor_a)))
    (Variables|Default|SetTarget_Angle 75.0)))

(event EventBeginPlay)

(event Collision|EventActorBeginOverlap
  (params (OtherActor :type Actor%20Object%20Reference)))

(event EventTick
  (params (DeltaSeconds :type Float%20%28single-precision%29))
  (bind _door_a (Variables|Default|GetDoor_a))
  (bind _target_angle (Variables|Default|GetTarget_Angle))
  (bind _relativerotation (Variables|/Script/Engine.SceneComponent|GetRelativeRotation _door_a))
  (bind _returnvalue (- (.yaw _relativerotation) _target_angle))
  (if (> (Math|Float|Absolute(Float) _returnvalue) (Variables|Default|GetThreshold))
    (Transformation|AddRelativeRotation (Variables|Default|GetDoor_a) (Math|Rotator|MakeRotator 0.0 0.0 (* DeltaSeconds (Variables|Default|GetSpeed) (Math|Float|Sign(Float) _returnvalue))) false false)
    (else
      (Transformation|SetRelativeRotation (Variables|Default|GetDoor_a) (Math|Rotator|MakeRotator 0.0 0.0 (Variables|Default|GetTarget_Angle)) false false))))

(fn ConstructionScript)